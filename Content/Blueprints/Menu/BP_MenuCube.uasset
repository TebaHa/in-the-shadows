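; Main menu cube actor with clickable faces for play, go back and choosing the Easy, Medium or Hard level.
; BeginPlay loads or creates the save, using completion flags to unlock Medium and Hard in sequence.
; Play and Goback flip the cube with Timelines behind a busy lock, while PlayTest flips it with all levels unlocked.
; Hover recolors labels, with completed levels shown differently, and Tick bobs the cube vertically.
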(event OnClicked(easybox)
  (params (TouchedComponent :type Primitive%20Component%20Object%20Reference) (ButtonPressed :type Key%20Structure :default "None"))
  (Game|OpenLevel(byName) "Level_Easy"))

(event OnClicked(mediumbox)
  (params (TouchedComponent :type Primitive%20Component%20Object%20Reference) (ButtonPressed :type Key%20Structure :default "None"))
  (Game|OpenLevel(byName) "Level_Medium"))

(event OnEndCursorOver(mediumbox)
  (params (TouchedComponent :type Primitive%20Component%20Object%20Reference))
  (CallFunction|MouseonOutFocus (Variables|Default|GetMedium)))

(event OnBeginCursorOver(hardbox)
  (params (TouchedComponent :type Primitive%20Component%20Object%20Reference))
  (CallFunction|MouseonFocus (Variables|Default|Gethard) (Variables|Default|GetIsHard)))

(event OnEndCursorOver(hardbox)
  (params (TouchedComponent :type Primitive%20Component%20Object%20Reference))
  (CallFunction|MouseonOutFocus (Variables|Default|Gethard)))

(event OnClicked(playbox)
  (params (TouchedComponent :type Primitive%20Component%20Object%20Reference) (ButtonPressed :type Key%20Structure :default "None"))
  (bind _hardbox (Variables|Default|Gethardbox))
  (bind _mediumbox (Variables|Default|Getmediumbox))
  (bind _cube (Variables|Default|GetCube))
  (if (not (Variables|Default|GetIsBusy))
    (Variables|Default|SetIsBusy true)
    (if (Variables|Default|GetIsEasy)
      (Collision|SetCollisionEnabled _mediumbox "QueryAndPhysics")
      (else
        (Collision|SetCollisionEnabled _mediumbox "NoCollision")))
    (if (Variables|Default|GetIsMedium)
      (Collision|SetCollisionEnabled _hardbox "QueryAndPhysics")
      (bind _newtrack_0 (Timeline|Timeline_0 PlayFromStart)
        (:Update
          (Transformation|AddLocalRotation _cube (Math|Rotator|MakeRotator 0.0 (* _newtrack_0 1.0) 0.0) false false))
        (:Finished
          (Variables|Default|SetIsBusy false)
          (Transformation|SetRelativeRotation _cube "90.000000, 0, 0" false false)))
      (else
        (Collision|SetCollisionEnabled _hardbox "NoCollision")
        (Timeline|Timeline_0 PlayFromStart)))))

(event OnClicked(goback)
  (params (TouchedComponent :type Primitive%20Component%20Object%20Reference) (ButtonPressed :type Key%20Structure :default "None"))
  (bind _cube (Variables|Default|GetCube))
  (if (not (Variables|Default|GetIsBusy))
    (Variables|Default|SetIsBusy true)
    (bind _newtrack_0 (Timeline|Timeline_1 PlayFromStart)
      (:Update
        (Transformation|AddLocalRotation _cube (Math|Rotator|MakeRotator 0.0 (* _newtrack_0 -1.0) 0.0) false false))
      (:Finished
        (Variables|Default|SetIsBusy false)
        (Transformation|SetRelativeRotation _cube "0, 0, 0" false false)))))

(event OnClicked(playboxtest)
  (params (TouchedComponent :type Primitive%20Component%20Object%20Reference) (ButtonPressed :type Key%20Structure :default "None"))
  (bind _cube (Variables|Default|GetCube))
  (if (not (Variables|Default|GetIsBusy))
    (Variables|Default|SetIsBusy true)
    (Collision|SetCollisionEnabled (Variables|Default|Getmediumbox) "QueryAndPhysics")
    (Collision|SetCollisionEnabled (Variables|Default|Gethardbox) "QueryAndPhysics")
    (bind _newtrack_0 (Timeline|Timeline_2 PlayFromStart)
      (:Update
        (Transformation|AddLocalRotation _cube (Math|Rotator|MakeRotator 0.0 (* _newtrack_0 1.0) 0.0) false false))
      (:Finished
        (Variables|Default|SetIsBusy false)
        (Transformation|SetRelativeRotation _cube "90.000000, 0, 0" false false)))))

(event OnClicked(hardbox)
  (params (TouchedComponent :type Primitive%20Component%20Object%20Reference) (ButtonPressed :type Key%20Structure :default "None"))
  (Game|OpenLevel(byName) "Level_Hard"))

(event OnBeginCursorOver(playbox)
  (params (TouchedComponent :type Primitive%20Component%20Object%20Reference))
  (CallFunction|MouseonFocus (Variables|Default|GetPlay) false))

(event OnEndCursorOver(playbox)
  (params (TouchedComponent :type Primitive%20Component%20Object%20Reference))
  (CallFunction|MouseonOutFocus (Variables|Default|GetPlay)))

(event OnBeginCursorOver(playboxtest)
  (params (TouchedComponent :type Primitive%20Component%20Object%20Reference))
  (CallFunction|MouseonFocus (Variables|Default|GetPlayTest) false))

(event OnEndCursorOver(playboxtest)
  (params (TouchedComponent :type Primitive%20Component%20Object%20Reference))
  (CallFunction|MouseonOutFocus (Variables|Default|GetPlayTest)))

(event OnBeginCursorOver(easybox)
  (params (TouchedComponent :type Primitive%20Component%20Object%20Reference))
  (CallFunction|MouseonFocus (Variables|Default|Getkeep%20warm) (Variables|Default|GetIsEasy)))

(event OnEndCursorOver(easybox)
  (params (TouchedComponent :type Primitive%20Component%20Object%20Reference))
  (CallFunction|MouseonOutFocus (Variables|Default|Getkeep%20warm)))

(event OnBeginCursorOver(mediumbox)
  (params (TouchedComponent :type Primitive%20Component%20Object%20Reference))
  (CallFunction|MouseonFocus (Variables|Default|GetMedium) (Variables|Default|GetIsMedium)))

(event EventBeginPlay
  (bind _mediumbox (Variables|Default|Getmediumbox))
  (bind _hardbox (Variables|Default|Gethardbox))
  (bind _mediumbox_2 (Variables|Default|Getmediumbox))
  (bind _hardbox_2 (Variables|Default|Gethardbox))
  (Utilities|FlowControl|Delay 1.0)
  (Audio|PlaySoundatLocation (Variables|Default|GetMainMenuMusic) (Transformation|GetActorLocation self) "0, 0, 0" 1.0 1.0 0.0 0 0 0)
  (bind _returnvalue (SaveGame|DoesSaveGameExist (Variables|Default|GetSaveFileName)))
  (if _returnvalue
    (bind _returnvalue_2 (SaveGame|LoadGamefromSlot (Variables|Default|GetSaveFileName)))
    (bind _asbp_save_game (Utilities|Casting|CastToBP_SaveGame _returnvalue_2))
    (Variables|Default|SetIsEasy (Variables|/Game/Blueprints/Menu/BP_SaveGame.BP_SaveGame_C|GetIsEasyLevelDone _asbp_save_game))
    (Variables|Default|SetIsMedium (Variables|/Game/Blueprints/Menu/BP_SaveGame.BP_SaveGame_C|GetIsMediumLevelDone _asbp_save_game))
    (Variables|Default|SetIsHard (Variables|/Game/Blueprints/Menu/BP_SaveGame.BP_SaveGame_C|GetIsHardLevelDone _asbp_save_game))
    (if (Variables|/Game/Blueprints/Menu/BP_SaveGame.BP_SaveGame_C|GetIsEasyLevelDone _asbp_save_game)
      (Collision|SetCollisionEnabled _mediumbox "QueryAndPhysics")
      (else
        (Collision|SetCollisionEnabled _mediumbox "NoCollision")))
    (if (Variables|/Game/Blueprints/Menu/BP_SaveGame.BP_SaveGame_C|GetIsMediumLevelDone _asbp_save_game)
      (Collision|SetCollisionEnabled _hardbox "QueryAndPhysics")
      (else
        (Collision|SetCollisionEnabled _hardbox "NoCollision")))
    (else
      (bind _returnvalue_3 (SaveGame|CreateSaveGameObject "/Game/Blueprints/Menu/BP_SaveGame.BP_SaveGame_C"))
      (Variables|Default|SetIsEasy (Variables|/Game/Blueprints/Menu/BP_SaveGame.BP_SaveGame_C|GetIsEasyLevelDone _returnvalue_3))
      (Variables|Default|SetIsMedium (Variables|/Game/Blueprints/Menu/BP_SaveGame.BP_SaveGame_C|GetIsMediumLevelDone _returnvalue_3))
      (Variables|Default|SetIsHard (Variables|/Game/Blueprints/Menu/BP_SaveGame.BP_SaveGame_C|GetIsHardLevelDone _returnvalue_3))
      (if (Variables|/Game/Blueprints/Menu/BP_SaveGame.BP_SaveGame_C|GetIsEasyLevelDone _returnvalue_3)
        (Collision|SetCollisionEnabled _mediumbox_2 "QueryAndPhysics")
        (else
          (Collision|SetCollisionEnabled _mediumbox_2 "NoCollision")))
      (if (Variables|/Game/Blueprints/Menu/BP_SaveGame.BP_SaveGame_C|GetIsMediumLevelDone _returnvalue_3)
        (Collision|SetCollisionEnabled _hardbox_2 "QueryAndPhysics")
        (else
          (Collision|SetCollisionEnabled _hardbox_2 "NoCollision")))
      (SaveGame|SaveGametoSlot _returnvalue_3 (Variables|Default|GetSaveFileName)))))

(event Collision|EventActorBeginOverlap
  (params (OtherActor :type Actor%20Object%20Reference)))

(event EventTick
  (params (DeltaSeconds :type Float%20%28single-precision%29))
  (bind _delta (Variables|Default|GetDelta))
  (if (>= (Variables|Default|GetAccum) 3.3)
    (Variables|Default|SetRotation (* -1 _delta))
    (elif (<= (Variables|Default|GetAccum) -2.8)
      (Variables|Default|SetRotation _delta)))
  (Transformation|AddRelativeLocation (Variables|Default|GetCube) (Math|Vector|MakeVector 0.0 0.0 (Variables|Default|GetRotation)) false false)
  (Variables|Default|SetAccum (+ (Variables|Default|GetRotation) (Variables|Default|GetAccum))))

(fn ConstructionScript)

(fn MouseonFocus
  (params (Text :type Text%20Render%20Component%20Object%20Reference) (IsDone :type Boolean))
  (if IsDone
    (Rendering|Components|TextRender|SetTextRenderColor Text (Math|Conversions|ToColor(LinearColor) "(R=0.000000,G=0.000000,B=0.000000,A=1.000000)"))
    (else
      (Rendering|Components|TextRender|SetTextRenderColor Text (Math|Conversions|ToColor(LinearColor) (Math|Color|MakeColor 255.0 255.0 255.0))))))

(fn MouseonOutFocus
  (params (Text :type Text%20Render%20Component%20Object%20Reference))
  (Rendering|Components|TextRender|SetTextRenderColor Text (Math|Conversions|ToColor(LinearColor) (Math|Color|MakeColor 255.0 0.0 0.0))))