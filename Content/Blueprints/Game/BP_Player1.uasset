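; Player Blueprint for the medium shadow-puzzle level, where two tagged objects are rotated into a target orientation.
; Left-drag rotates the object under the cursor by line trace in world yaw, or pitch while Left Ctrl is held.
; When not dragging, Tick compares both rotations against hardcoded tolerances and times the match.
; A sustained match saves completion and spawns the congrats widget every tick, then soon lets a click open the main menu.
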(event EventBeginPlay
  (bind _outactors (Actor|GetAllActorsOfClasswithTag (Variables|Default|GetPuzzleClass) "Puzzle1"))
  (Variables|Default|SetPuzzleActor (Utilities|Array|Get(acopy) _outactors))
  (bind _outactors_2 (Actor|GetAllActorsOfClasswithTag (Variables|Default|GetPuzzleClass1) "Puzzle2"))
  (Variables|Default|SetPuzzleActor1 (Utilities|Array|Get(acopy) _outactors_2)))

(event Collision|EventActorBeginOverlap
  (params (OtherActor :type Actor%20Object%20Reference)))

(event EventTick
  (params (DeltaSeconds :type Float%20%28single-precision%29))
  (bind _puzzleactor (Variables|Default|GetPuzzleActor))
  (bind _puzzleactor1 (Variables|Default|GetPuzzleActor1))
  (bind _rotateactor (Variables|Default|GetRotateActor))
  (bind _returnvalue (Transformation|GetActorRotation _puzzleactor))
  (bind _returnvalue_2 (Transformation|GetActorRotation _puzzleactor1))
  (bind (_roll _pitch _yaw) (Math|Rotator|BreakRotator _returnvalue))
  (bind (_roll_2 _pitch_2 _yaw_2) (Math|Rotator|BreakRotator _returnvalue_2))
  (if (Variables|Default|GetIsDraggin)
    (if (Variables|Default|GetIsHor)
      (bind _output_get (Variables|Default|SetSum_Y (- (Variables|Default|GetSum_Y) (Class|Actor|GetInputAxisKeyValue))))
      (Class|Actor|AddActorWorldRotation _rotateactor (Math|Rotator|MakeRotator 0.0 (* (* _output_get DeltaSeconds) 12.0) 0.0))
      (else
        (bind _output_get_2 (Variables|Default|SetSum_X (- (Variables|Default|GetSum_X) (Class|Actor|GetInputAxisKeyValue))))
        (Class|Actor|AddActorWorldRotation _rotateactor (Math|Rotator|MakeRotator 0.0 0.0 (* (* _output_get_2 DeltaSeconds) 12.0)))))
    (elif (Math|Boolean|ANDBoolean (Math|Float|NearlyEqual(Float) _roll 93.5 15.0) (Math|Float|NearlyEqual(Float) _pitch 2.0 15.0) (Math|Float|NearlyEqual(Float) _yaw 165.0 15.0) (Math|Float|NearlyEqual(Float) _roll_2 -92.0 1.5e+02) (Math|Float|NearlyEqual(Float) _pitch_2 -2.2 15.0) (Math|Float|NearlyEqual(Float) _yaw_2 -18.700001 15.0))
      (bind _output_get_3 (Variables|Default|SetTimeAccum (+ (Variables|Default|GetTimeAccum) DeltaSeconds)))
      (if (> _output_get_3 6.0)
        (bind _returnvalue_3 (SaveGame|DoesSaveGameExist "InTheShadowsSave"))
        (if _returnvalue_3
          (bind _returnvalue_4 (SaveGame|LoadGamefromSlot "InTheShadowsSave"))
          (bind _asbp_save_game (Utilities|Casting|CastToBP_SaveGame _returnvalue_4))
          (Variables|/Game/Blueprints/Menu/BP_SaveGame.BP_SaveGame_C|SetIsMediumLevelDone _asbp_save_game true)
          (SaveGame|SaveGametoSlot _asbp_save_game "InTheShadowsSave"))
        (bind _returnvalue_5 (UserInterface|CreateWidget "/Game/UI/WG_Congrats.WG_Congrats_C" (Game|GetPlayerController 0)))
        (UserInterface|Viewport|AddtoViewport _returnvalue_5 0)
        (Default|SetActive _returnvalue_5)
        (if (> (Variables|Default|GetTimeAccum) 8.0)
          (Variables|Default|SetIsWin true)))
      (else
        (Variables|Default|SetTimeAccum 0.0)))))

(event Input|KeyboardEvents|LeftCtrl
  (params (Key :type Key%20Structure :default "None"))
  (:Pressed
    (Variables|Default|SetIsHor true))
  (:Released
    (Variables|Default|SetIsHor false)))

(event Input|MouseEvents|LeftMouseButton
  (params (Key :type Key%20Structure :default "None"))
  (bind _returnvalue (Game|GetPlayerController 0))
  (bind (_worldlocation _worlddirection) (Game|Player|ConvertMouseLocationToWorldSpace _returnvalue))
  (:Pressed
    (if (Variables|Default|GetIsWin)
      (Game|OpenLevel(byName) "Level_MainMenu")
      (else
        (bind (_outhit _returnvalue_2) (Collision|LineTraceByChannel _worldlocation (+ _worldlocation (* _worlddirection 1.5e+03)) "TraceTypeQuery1" false 0 "None"))
        (if _returnvalue_2
          (Variables|Default|SetRotateActor (.HitActor (Collision|BreakHitResult _outhit)))
          (Variables|Default|SetIsDraggin true)))))
  (:Released
    (Variables|Default|SetIsDraggin false)
    (Variables|Default|SetSum_X 0.0)
    (Variables|Default|SetSum_Y 0.0)))

(fn ConstructionScript)