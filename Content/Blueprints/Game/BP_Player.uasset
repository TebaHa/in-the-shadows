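; Player Blueprint for a rotation puzzle level, turning the "Puzzle"-tagged actor by left-mouse drag.
; Tick yaws the actor from accumulated axis input while dragging, otherwise times how long it rests near the target yaw.
; After a short hold it flags the easy level done in any existing save and adds a congrats widget every tick.
; A longer hold sets IsWin, making the next click open the main menu.
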(event EventBeginPlay
  (bind _outactors (Actor|GetAllActorsOfClasswithTag (Variables|Default|GetPuzzleClass) "Puzzle"))
  (Variables|Default|SetPuzzleActor (Utilities|Array|Get(acopy) _outactors)))

(event Collision|EventActorBeginOverlap
  (params (OtherActor :type Actor%20Object%20Reference)))

(event EventTick
  (params (DeltaSeconds :type Float%20%28single-precision%29))
  (if (Variables|Default|GetIsDraggin)
    (bind _output_get (Variables|Default|SetSum_X (- (Variables|Default|GetSum_X) (Class|Actor|GetInputAxisKeyValue))))
    (Class|Actor|AddActorWorldRotation (Variables|Default|GetPuzzleActor) (Math|Rotator|MakeRotator 0.0 0.0 (* (* _output_get DeltaSeconds) 12.0)))
    (elif (Math|Float|NearlyEqual(Float) (.Yaw (Math|Rotator|BreakRotator (Transformation|GetActorRotation (Variables|Default|GetPuzzleActor)))) 6e+01 5.0)
      (bind _output_get_2 (Variables|Default|SetTimeAccum (+ (Variables|Default|GetTimeAccum) DeltaSeconds)))
      (if (> _output_get_2 3.0)
        (bind _returnvalue (SaveGame|DoesSaveGameExist "InTheShadowsSave"))
        (Development|PrintString (Utilities|String|ToString(Boolean) _returnvalue))
        (if _returnvalue
          (bind _returnvalue_2 (SaveGame|LoadGamefromSlot "InTheShadowsSave"))
          (bind _asbp_save_game (Utilities|Casting|CastToBP_SaveGame _returnvalue_2))
          (Variables|/Game/Blueprints/Menu/BP_SaveGame.BP_SaveGame_C|SetIsEasyLevelDone _asbp_save_game true)
          (SaveGame|SaveGametoSlot _asbp_save_game "InTheShadowsSave"))
        (bind _returnvalue_3 (UserInterface|CreateWidget "/Game/UI/WG_Congrats.WG_Congrats_C" (Game|GetPlayerController 0)))
        (UserInterface|Viewport|AddtoViewport _returnvalue_3 0)
        (Default|SetActive _returnvalue_3)
        (if (> (+ (Variables|Default|GetTimeAccum) DeltaSeconds) 6.0)
          (Variables|Default|SetIsWin true)))
      (else
        (Variables|Default|SetTimeAccum 0.0)))))

(event Input|MouseEvents|LeftMouseButton
  (params (Key :type Key%20Structure :default "None"))
  (:Pressed
    (if (Variables|Default|GetIsWin)
      (Game|OpenLevel(byName) "Level_MainMenu")
      (else
        (Variables|Default|SetIsDraggin true))))
  (:Released
    (Variables|Default|SetIsDraggin false)
    (Variables|Default|SetSum_X 0.0)
    (Variables|Default|SetSum_Y 0.0)))

(fn ConstructionScript)